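; Boss enemy that picks a melee or ranged attack by player distance and shows its health on a screen widget.
; Close attacks damage whatever pawn a forward box trace hits; distant ones spawn and throw a projectile on a montage notify.
; An Attacking flag plus a post-montage delay gates both attacks.
; Death enables physics on the mesh and stops WheelMoving, while UpdateHealthBar feeds Health to the widget.
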(event `self.ReceiveBeginPlay`
  (set `self.AIController` (`AIBlueprintHelperLibrary.GetAIController` self))
  (bind _returnvalue (`|CreateWidget` "/Game/UI/BossHealthBar.BossHealthBar_C"))
  (bind _output_get (set `self.BossHealthBar` _returnvalue))
  (`UserWidget.AddToViewport` _output_get 0))

(event `Boss_Attack`
  (bind _returnvalue (`self.K2_GetActorLocation`))
  ;[1 1 1 0.5] Attack
  (if (> (`KismetMathLibrary.Vector_Distance` (`self.K2_GetActorLocation`) (`self.K2_GetActorLocation` (`GameplayStatics.GetPlayerCharacter` 0))) 700.0)
    (`self.Boss_Attack_Range`)
    (elif (not (`self.Attacking`))
      (`|PlayMontage` (`self.Mesh`) "/Game/Ancient_Golem/Demo/ThirdPersonJump_Start_Montage.ThirdPersonJump_Start_Montage"
        (:`then`
          (set `self.Attacking` true)
          (`GameplayStatics.PlaySoundAtLocation` "/Engine/EditorSounds/GamePreview/StartPlayInEditor_Cue.StartPlayInEditor_Cue" _returnvalue (struct) 1.0 1.0 1.0 "/USDCore/USDDefaultAttenuation.USDDefaultAttenuation" null null null)
          (bind (_outhit _returnvalue_2) (`KismetSystemLibrary.BoxTraceSingleForObjects` _returnvalue (+ _returnvalue (* (`self.GetActorForwardVector`) 400.0)) (75.0 200.0 100.0) (struct) (`|MakeArray` "ObjectTypeQuery3" :!type "EObjectTypeQuery Enum")))
          (if _returnvalue_2
            (`GameplayStatics.ApplyDamage` (`.HitActor` (`GameplayStatics.BreakHitResult` _outhit)) 34.0)))
        (:`OnCompleted`
          (`KismetSystemLibrary.Delay` 1.0)
          (set `self.Attacking` false))))))

(event `Boss_Attack_Range`
  (bind _returnvalue (`SceneComponent.K2_GetComponentLocation` (`self.ProjectileLocation`)))
  ;[1 1 1 0.5] Ranged Attack
  (if (not (`self.Attacking`))
    (`|PlayMontage` (`self.Mesh`) "/Game/Ancient_Golem/Demo/ThirdPersonJump_Start_Montage.ThirdPersonJump_Start_Montage"
      (:`then`
        (set `self.Attacking` true)
        (`GameplayStatics.PlaySoundAtLocation` "/Engine/VREditor/Sounds/UI/Teleport_Committed.Teleport_Committed" _returnvalue (struct) 1.0 1.0 0.0 "/USDCore/USDDefaultAttenuation.USDDefaultAttenuation" null null null))
      (:`OnCompleted`
        (`KismetSystemLibrary.Delay` 1.0)
        (set `self.Attacking` false))
      (:`OnNotifyBegin`
        (bind _returnvalue_2 (`|SpawnActorFromClass` "/Game/Enemies/Boss/BP_Boss_Projectile.BP_Boss_Projectile_C" (`KismetMathLibrary.MakeTransform` _returnvalue) "Undefined" "MultiplyWithRoot" null null))
        (`/Game/Enemies/Boss/BP_Boss_Projectile.Throw` _returnvalue_2)))))

(fn `Death`
  (bind _mesh (`self.Mesh`))
  (`PrimitiveComponent.SetSimulatePhysics` _mesh true)
  (`PrimitiveComponent.SetCollisionEnabled` _mesh "QueryAndPhysics")
  (`SkeletalMeshComponent.Stop` (`self.WheelMoving`)))

(fn `UpdateHealthBar`
  (bind _bosshealthbar (`self.BossHealthBar`))
  (if (`KismetSystemLibrary.IsValid` _bosshealthbar)
    (`ProgressBar.SetPercent` (`/Game/UI/BossHealthBar.BossHB` _bosshealthbar) (/ (`self.Health`) 500.0))))

(fn `UserConstructionScript`)