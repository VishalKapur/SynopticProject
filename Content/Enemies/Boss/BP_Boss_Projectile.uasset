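; BP_Boss_Projectile is a projectile for the boss that damages the first-person player on contact.
; A Throw event sets the player's capsule as the ProjectileMovement homing target.
; Box overlaps ignore BP_Boss, apply damage only to BP_FirstPersonCharacter and then destroy the projectile.
; The projectile also destroys itself after a fixed delay from BeginPlay.
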(event `self.ReceiveBeginPlay`
  (`KismetSystemLibrary.Delay` 10.0)
  (`self.K2_DestroyActor`))

(event `Throw`
  (set `ProjectileMovementComponent.HomingTargetComponent` (`self.GetComponentByClass` (`GameplayStatics.GetPlayerCharacter` 0) "/Script/Engine.CapsuleComponent") (`self.ProjectileMovement`)))

(event `self.Box.OnComponentBeginOverlap`
  (params (OverlappedComponent :type "PrimitiveComponent Object Reference") (OtherActor :type "Actor Object Reference") (OtherComp :type "PrimitiveComponent Object Reference") (OtherBodyIndex :type Integer) (bFromSweep :type Boolean) (SweepResult :type "HitResult Structure (by ref)"))
  (cast `/Game/Enemies/Boss/BP_Boss` OtherActor
    (:`CastFailed`
      (cast `/Game/FirstPerson/Blueprints/BP_FirstPersonCharacter` OtherActor)
      (`GameplayStatics.ApplyDamage` OtherActor 20.0)
      (`self.K2_DestroyActor`))))

(fn `UserConstructionScript`)