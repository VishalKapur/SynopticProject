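; BP_Enemy is a melee enemy character with a floating health bar that rotates toward the player camera every Tick.
; Attack plays a montage if none is running, then after a short delay sphere-traces forward for pawns and damages the hit actor, with debug drawing on.
; UpdateHealthBar writes Health to the widget as a percentage.
; Death ragdolls the mesh and destroys the capsule and health bar.
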(event `self.ReceiveTick`
  (params (DeltaSeconds :type "Float (single-precision)"))
  (bind _health_bar (`self.Health Bar`))
  (if (`KismetSystemLibrary.IsValid` _health_bar)
    (`SceneComponent.K2_SetWorldRotation` _health_bar (`KismetMathLibrary.FindLookAtRotation` (`SceneComponent.K2_GetComponentLocation` _health_bar) (`SceneComponent.K2_GetComponentLocation` (`PlayerCameraManager.TransformComponent` (`GameplayStatics.GetPlayerCameraManager` 0)))) false false)))

(event `Attack`
  (bind _returnvalue (`self.K2_GetActorLocation`))
  (bind _mesh (`self.Mesh`))
  ;[1 1 1 0.5] Attack
  (if (not (`AnimInstance.IsAnyMontagePlaying` (`SkeletalMeshComponent.GetAnimInstance` _mesh)))
    (`|PlayMontage` _mesh "/Game/Animations/EnemyAttackMontage.EnemyAttackMontage"
      (:`then`
        (`KismetSystemLibrary.Delay` 0.7)
        (bind (_outhit _returnvalue_2) (`KismetSystemLibrary.SphereTraceSingleForObjects` :`Start` _returnvalue :`End` (+ _returnvalue (* (`self.GetActorForwardVector`) 200.0)) :`Radius` 50.0 :`ObjectTypes` (`|MakeArray` "ObjectTypeQuery3" :!type "EObjectTypeQuery Enum") :`DrawDebugType` "ForDuration"))
        (if _returnvalue_2
          (`GameplayStatics.ApplyDamage` (`.HitActor` (`GameplayStatics.BreakHitResult` _outhit)) 20.0))))))

(fn `Death`
  (bind _mesh (`self.Mesh`))
  (`PrimitiveComponent.SetSimulatePhysics` _mesh true)
  (`PrimitiveComponent.SetCollisionEnabled` _mesh "QueryAndPhysics")
  (`ActorComponent.K2_DestroyComponent` (`self.CapsuleComponent`))
  (`ActorComponent.K2_DestroyComponent` (`self.Health Bar`)))

(fn `UpdateHealthBar`
  (bind _asenemy_health_bar (cast `/Game/UI/EnemyHealthBar` (`WidgetComponent.GetWidget` (`self.Health Bar`))))
  (if (`KismetSystemLibrary.IsValid` _asenemy_health_bar)
    (`ProgressBar.SetPercent` (`/Game/UI/EnemyHealthBar.EnemyHB` _asenemy_health_bar) (/ (`self.Health`) 100.0))))

(fn `UserConstructionScript`)