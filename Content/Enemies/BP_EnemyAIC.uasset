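; Enemy AI controller that runs the BT_Enemy behavior tree and feeds it player sightings.
; PawnSensing writes a seen Player-tagged pawn and its location to the blackboard as target and destination.
; Every sighting, of any pawn, restarts a one-second retriggerable delay that clears the target when sightings stop, leaving the last destination in place.
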(event `self.ReceiveBeginPlay`
  (`self.RunBehaviorTree` "/Game/Enemies/BT_Enemy.BT_Enemy"))

(event `self.PawnSensing.OnSeePawn`
  (params (Pawn :type "Pawn Object Reference"))
  (bind _returnvalue (`AIBlueprintHelperLibrary.GetBlackboard` null))
  (bind _blackboardkeytarget (`self.BlackboardKeyTarget`))
  ;[1 1 1 0.5] Chase Player
  (`|ExecutionSequence`
    (:`then_0`
      (if (`self.ActorHasTag` Pawn "Player")
        (`BlackboardComponent.SetValueAsVector` _returnvalue (`self.BlackboardKeyDestination`) (`self.K2_GetActorLocation` Pawn))
        (`BlackboardComponent.SetValueAsObject` _returnvalue _blackboardkeytarget Pawn)))
    (:`then_1`
      ;;[1 1 1 0.5] Lost Sight
      (`KismetSystemLibrary.RetriggerableDelay` 1.0)
      (`BlackboardComponent.ClearValue` _returnvalue _blackboardkeytarget))))

(fn `UserConstructionScript`)