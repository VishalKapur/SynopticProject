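; Base enemy Blueprint that tracks health and takes damage from standard damage events and physical impacts.
; Hits from actors tagged DamageObject with enough downward normal impulse feed a fixed damage amount into the same path as AnyDamage.
; That path subtracts health, updates the health bar and calls Death once health runs out.
; Death and UpdateHealthBar are empty here, as are construction, BeginPlay and Tick.
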(event `self.ReceiveAnyDamage`
  (params (Damage :type "Float (single-precision)") (DamageType :type "DamageType Object Reference") (InstigatedBy :type "Controller Object Reference") (DamageCauser :type "Actor Object Reference"))
  (bind _health (`self.Health`))
  ;[1 1 1 0.5] Health
  (set `self.Damage` Damage)
  (set `self.Health` (- _health (`self.Damage`)) :!label _label)
  (`self.UpdateHealthBar`)
  (if (<= _health 0.0)
    (`self.Death`)))

(event `self.ReceiveHit`
  (params (MyComp :type "PrimitiveComponent Object Reference") (Other :type "Actor Object Reference") (OtherComp :type "PrimitiveComponent Object Reference") (bSelfMoved :type Boolean) (HitLocation :type "Vector Structure") (HitNormal :type "Vector Structure") (NormalImpulse :type "Vector Structure") (Hit :type "HitResult Structure (by ref)"))
  ;[1 1 1 0.5] Health
  (if (and (`self.ActorHasTag` Other "DamageObject") (< NormalImpulse_Z -10.0))
    (set `self.Damage` 100.0)
    (goto _label)))

(fn `Death`)

(fn `UpdateHealthBar`)

(fn `UserConstructionScript`)