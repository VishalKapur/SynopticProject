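; BP_Flammable_Surface is a trap surface that catches fire and spreads it to neighboring flammable surfaces.
; Instances tagged "Start" ignite on BeginPlay, showing their fire effect and switching their nav modifier to an obstacle area.
; After a one-second delay, each calls SpreadFire on surfaces overlapping its SpreadRadius, creating a chain reaction.
; No burning-state check exists, so surfaces can be re-triggered by their neighbors.
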(event `self.ReceiveBeginPlay`
  (if (`self.ActorHasTag` "Start")
    (`self.SpreadFire`)))

(event `SpreadFire`
  (`SceneComponent.SetVisibility` (`self.Blueprint_Effect_Fire`) true false)
  (`NavModifierComponent.SetAreaClass` (`self.NavModifier`) "/Script/NavigationSystem.NavArea_Obstacle")
  (`KismetSystemLibrary.Delay` 1.0)
  (for _array_element (`PrimitiveComponent.GetOverlappingActors` (`self.SpreadRadius`) "BP_Flammable_Surface_C")
    (bind _asbp_flammable_surface (cast `/Game/Traps/BP_Flammable_Surface` _array_element))
    (`self.SpreadFire` _asbp_flammable_surface)))

(fn `UserConstructionScript`)